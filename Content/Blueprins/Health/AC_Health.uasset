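; Actor component that tracks health for its owning actor.
; On BeginPlay it fills Health to MaxHealth and binds to the owner's OnTakeAnyDamage event.
; GetDamagedEvent passes damage to GetDamaged, which subtracts it with a floor at zero.
; GetHeald checks the MaxHealth cap before adding healing, so a heal can push Health above the maximum.
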(event `self.ReceiveBeginPlay`
  (`|ExecutionSequence`
    (:`then_0`
      (set `self.Health` (`self.MaxHealth`)))
    (:`then_1`
      (add `Actor.OnTakeAnyDamage` (`self.GetOwner`) (`|CreateDelegate` :!event `GetDamagedEvent`)))))

(fn `GetDamaged`
  (params (Damage :type "Float (double-precision)"))
  (bind _returnvalue (- (`self.Health`) Damage))
  (if (>= _returnvalue 0.0)
    (set `self.Health` _returnvalue)
    (else
      (set `self.Health` 0.0))))

(fn `GetDamagedEvent`
  (params (DamagedActor :type "Actor Object Reference") (Damage :type "Float (single-precision)") (DamageType :type "DamageType Object Reference") (InstigatedBy :type "Controller Object Reference") (DamageCauser :type "Actor Object Reference"))
  (`self.GetDamaged` Damage))

(fn `GetHeald`
  (params (Heal :type "Float (double-precision)"))
  (if (> (`self.Health`) (`self.MaxHealth`))
    (set `self.Health` (`self.MaxHealth`))
    (else
      (set `self.Health` (+ (`self.Health`) Heal)))))